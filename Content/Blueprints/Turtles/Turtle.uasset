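; Turtle actor that moves forward until it overlaps its FinalDestination component, with flying audio started at spawn.
; Tick switches on TurtleType for steady movement, stop-and-go bursts with audio pauses, or forward runs with brief reversals, using accumulated timers and unscaled per-frame offsets.
; On arrival it stops ticking, plays hit audio, activates the DestinationReached effect, teleports the body far below to hide it and destroys itself after a delay.
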(event `self.ReceiveBeginPlay`
  ;[1 1 1] Make wind go from the beggining
  (`ActorComponent.Activate` (`self.Flying_Shot_Audio`) true))

(event `self.ReceiveTick`
  (params (DeltaSeconds :type "Float (single-precision)"))
  ;[1 1 1] Do movement.
  (`|ExecutionSequence`
    (:`then_0`
      (switch `/Game/Blueprints/Interaction/ButtonActions_enum` (`self.turtle_type`)
        (:`NewEnumerator0`
          ;[1 1 1] Turtle - 1 behavior
          (`SceneComponent.K2_AddWorldOffset` (`self.turtle_body`) (* (`SceneComponent.GetForwardVector` (`self.turtle_body`)) (`self.speed`)) false false))
        (:`NewEnumerator1`
          ;[1 1 1] Turtle - 2 behavior
          (if (< (`self.Timer_2_Turtle`) 1.0)
            (`SceneComponent.K2_AddWorldOffset` (`self.turtle_body`) (* (`SceneComponent.GetForwardVector` (`self.turtle_body`)) (`self.speed`)) false false)
            (set `self.Timer_2_Turtle` (+ (`self.Timer_2_Turtle`) (`GameplayStatics.GetWorldDeltaSeconds`)))
            (else
              (`ActorComponent.Deactivate` (`self.Flying_Shot_Audio`))
              (`KismetSystemLibrary.Delay` 0.5)
              (set `self.Timer_2_Turtle` 0.0)
              (`ActorComponent.Activate` (`self.Flying_Shot_Audio`) true))))
        (:`NewEnumerator2`
          ;[1 1 1] Turtle - 3 behavior
          (if (< (`self.Timer_3_Turtle`) 1.0)
            (`SceneComponent.K2_AddWorldOffset` (`self.turtle_body`) (* (`SceneComponent.GetForwardVector` (`self.turtle_body`)) (`self.speed`)) false false)
            (set `self.Timer_3_Turtle` (+ (`self.Timer_3_Turtle`) (`GameplayStatics.GetWorldDeltaSeconds`)))
            (else
              (`SceneComponent.K2_AddWorldOffset` (`self.turtle_body`) (* (* (`SceneComponent.GetForwardVector` (`self.turtle_body`)) (`self.speed`)) -1.0) false false)
              (set `self.Timer_3_MovingBackwards` (+ (`self.Timer_3_MovingBackwards`) (`GameplayStatics.GetWorldDeltaSeconds`)))
              (if (> (`self.Timer_3_MovingBackwards`) 0.5)
                (set `self.Timer_3_MovingBackwards` 0.0)
                (set `self.Timer_3_Turtle` 0.0)))))))
    (:`then_1`
      ;[1 1 1] Check for collision
      (if (`PrimitiveComponent.IsOverlappingComponent` (`self.turtle_body`) (`self.final_destination`))
        (`ActorComponent.Activate` (`self.Hit_Target_Audio`) true)
        (`self.SetActorTickEnabled` false)
        (`SceneComponent.K2_AddWorldOffset` (`self.turtle_body`) (0.0 0.0 -10000.0) false true)
        (`ActorComponent.SetActive` (`self.Destination_Reached`) true true)
        (`KismetSystemLibrary.Delay` 2.0)
        (`self.K2_DestroyActor`)))))

(fn `UserConstructionScript`)