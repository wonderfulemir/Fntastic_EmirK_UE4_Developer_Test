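; MainCharacter is the player character, with mouse look, WASD movement relative to control yaw, and button interaction.
; On Interact, a Visibility line trace runs from the capsule along the full control rotation out to InteractionRange.
; A hit Button plays its press sequence and the button audio activates on each press, while its action message fires only if it is not already Activated.
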(event `InputAxis|Look_UpDown`
  (params (AxisValue :type "Float (single-precision)"))
  ;[1 1 1] Looking with Mouse
  (`self.AddControllerPitchInput` AxisValue))

(event `InputAxis|Look_RightLeft`
  (params (AxisValue :type "Float (single-precision)"))
  ;[1 1 1] Looking with Mouse
  (`self.AddControllerYawInput` AxisValue))

(event `InputAxis|Move_ForwardBackward`
  (params (AxisValue :type "Float (single-precision)"))
  (bind (_returnvalue_roll _returnvalue_pitch _returnvalue_yaw) (`KismetMathLibrary.BreakRotator` (`self.GetControlRotation`)))
  ;[1 1 1] Movement with WASD
  (`self.AddMovementInput` (`KismetMathLibrary.GetForwardVector` (`KismetMathLibrary.MakeRotator` 0.0 0.0 _returnvalue_yaw)) AxisValue))

(event `InputAxis|Move_LeftRight`
  (params (AxisValue :type "Float (single-precision)"))
  (bind (_returnvalue_roll _returnvalue_pitch _returnvalue_yaw) (`KismetMathLibrary.BreakRotator` (`self.GetControlRotation`)))
  ;[1 1 1] Movement with WASD
  (`self.AddMovementInput` (`KismetMathLibrary.GetRightVector` (`KismetMathLibrary.MakeRotator` 0.0 0.0 _returnvalue_yaw)) AxisValue))

(event `InputAction|Interact`
  (params (Key :type "Key Structure"))
  (bind (_returnvalue_roll _returnvalue_pitch _returnvalue_yaw) (`KismetMathLibrary.BreakRotator` (`self.GetControlRotation`)))
  (bind _returnvalue (`SceneComponent.K2_GetComponentLocation` (`self.CapsuleComponent`)))
  ;[1 1 1] Interacting with Buttons
  (:`Pressed`
    (bind _outhit (`KismetSystemLibrary.LineTraceSingle` _returnvalue (+ _returnvalue (* (`KismetMathLibrary.GetForwardVector` (`KismetMathLibrary.MakeRotator` _returnvalue_roll _returnvalue_pitch _returnvalue_yaw)) (`self.InteractionRange`))) "TraceTypeQuery1"))
    (bind _asbutton (cast `/Game/Blueprints/Interaction/Button` (`.HitActor` (`GameplayStatics.BreakHitResult` _outhit))))
    (`MovieSceneSequencePlayer.Play` (`ActorSequenceComponent.SequencePlayer` (`/Game/Blueprints/Interaction/Button.PressedSequence` _asbutton)))
    (`ActorComponent.Activate` (`self.Button_Audio`) true)
    (if (not (`/Game/Blueprints/Interaction/Button.Activated` _asbutton))
      (message `/Game/Blueprints/Interaction/Button_BP_Interface.Do_Button_Action` _asbutton))))

(fn `UserConstructionScript`)