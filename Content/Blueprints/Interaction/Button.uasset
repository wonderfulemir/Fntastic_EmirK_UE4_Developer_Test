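; Interactable button Blueprint that spawns a Turtle when its DoButtonAction event fires.
; The Turtle appears at the TurtleHome component's transform and receives its TurtleType from the button's MyActionEnum.
; The event also sets an Activated flag and shows and restarts the Shot effect, then clears both after a Cooldown delay.
; The event itself does not check Activated before spawning.
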(event `/Game/Blueprints/Interaction/Button_BP_Interface.Do_Button_Action`
  (set `self.Activated` true)
  (bind _returnvalue (`|SpawnActorFromClass` "/Game/Blueprints/Turtles/Turtle.Turtle_C" (`SceneComponent.K2_GetComponentToWorld` (`self.Turtle_Home`)) "Undefined" "OverrideRootScale" null null))
  (set `/Game/Blueprints/Turtles/Turtle.turtle_type` (`self.MyActionEnum`) _returnvalue)
  (`SceneComponent.SetVisibility` (`self.Shot`) true false)
  (`NiagaraComponent.ResetSystem` (`self.Shot`))
  (`KismetSystemLibrary.Delay` (`self.Cooldown`))
  (set `self.Activated` false)
  (`SceneComponent.SetVisibility` (`self.Shot`) false false))

(fn `UserConstructionScript`)